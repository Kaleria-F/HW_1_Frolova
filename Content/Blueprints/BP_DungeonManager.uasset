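; BP_DungeonManager is a dungeon manager actor with an unfinished GenerateRooms function for placing BP_Room actors.
; Each call spawns one scaled, rotated room at a fixed Y offset from the given location, unless CurrentRoomIndex plus one equals the requested amount.
; RoomArray is overwritten with just that room.
; There is no loop or index increment, the previous-location update is disconnected, and no event calls the function.
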(event EventBeginPlay)

(event Collision|EventActorBeginOverlap
  (params (OtherActor :type Actor%20Object%20Reference)))

(event EventTick
  (params (DeltaSeconds :type Float%20%28single-precision%29)))

(fn ConstructionScript)

(fn GenerateRooms
  (params (PLocation :type Vector) (AmountRooms :type Integer))
  (if (not (== (+ (Variables|Default|GetCurrentRoomIndex%20) 1) AmountRooms))
    (bind _returnvalue (Game|SpawnActorfromClass "/Game/Blueprints/BP_Room.BP_Room_C" (Math|Transform|MakeTransform (+ PLocation (Math|Vector|MakeVector 0.0 7.8e+02 0.0)) "0.000000,-90.000000,0.000000" "3.500000,3.500000,3.500000") "Undefined" "MultiplyWithRoot" 0 0))
    (Variables|Default|SetRoomArray (Utilities|Array|MakeArray _returnvalue))))