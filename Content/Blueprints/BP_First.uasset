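; BP_First is a dungeon room with two exits that pick a Light or Hard difficulty for room generation.
; BeginPlay stores the room's location.
; When the player overlaps an exit, it writes the room count to the character and tells BP_DungeonManager to generate rooms from that location.
; The Hard exit also spawns snail and recover traps at fixed transforms.
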(event OnComponentBeginOverlap(Exit1)
  (params (OverlappedComponent :type Primitive%20Component%20Object%20Reference) (OtherActor :type Actor%20Object%20Reference) (OtherComp :type Primitive%20Component%20Object%20Reference) (OtherBodyIndex :type Integer) (bFromSweep :type Boolean) (SweepResult :type Hit%20Result%20Structure%20%28by%20ref%29))
  (Utilities|Casting|CastToBP_ThirdPersonCharacter OtherActor)
  (Development|PrintString "Light")
  (bind _outactors (Actor|GetAllActorsOfClass "/Game/Blueprints/BP_DungeonManager.BP_DungeonManager_C"))
  (CallFunction|InitializeRoom)
  (Default|GenerateRooms (Utilities|Array|Get(acopy) _outactors) (Variables|Default|GetRoomLocation) (Variables|Default|GetFinishRoom) (Variables|Default|GetLight)))

(event OnComponentBeginOverlap(Exit2)
  (params (OverlappedComponent :type Primitive%20Component%20Object%20Reference) (OtherActor :type Actor%20Object%20Reference) (OtherComp :type Primitive%20Component%20Object%20Reference) (OtherBodyIndex :type Integer) (bFromSweep :type Boolean) (SweepResult :type Hit%20Result%20Structure%20%28by%20ref%29))
  (Utilities|Casting|CastToBP_ThirdPersonCharacter OtherActor)
  (Development|PrintString "Hard")
  (Game|SpawnActorfromClass (Utilities|GetClass (Variables|Default|GetSnailTrapClass%20)) (Math|Transform|MakeTransform "-79.000000,-94.000000,0.000000") "Undefined" "MultiplyWithRoot" 0 0)
  (Game|SpawnActorfromClass (Utilities|GetClass (Variables|Default|GetRecoverTrapClass%20)) (Math|Transform|MakeTransform "0, 0, 0") "Undefined" "MultiplyWithRoot" 0 0)
  (bind _outactors (Actor|GetAllActorsOfClass "/Game/Blueprints/BP_DungeonManager.BP_DungeonManager_C"))
  (CallFunction|InitializeRoom)
  (Default|GenerateRooms (Utilities|Array|Get(acopy) _outactors) (Variables|Default|GetRoomLocation) (Variables|Default|GetFinishRoom) (Variables|Default|GetHard)))

(event EventBeginPlay
  (Variables|Default|SetRoomLocation (Transformation|GetActorLocation)))

(event Collision|EventActorBeginOverlap
  (params (OtherActor :type Actor%20Object%20Reference)))

(event EventTick
  (params (DeltaSeconds :type Float%20%28single-precision%29)))

(fn ConstructionScript)

(fn InitializeRoom
  (bind _outactors (Actor|GetAllActorsOfClass "/Game/ThirdPerson/Blueprints/BP_ThirdPersonCharacter.BP_ThirdPersonCharacter_C"))
  (Variables|/Game/ThirdPerson/Blueprints/BP_ThirdPersonCharacter.BP_ThirdPersonCharacter_C|SetAmountRoomsGlob (Utilities|Array|Get(acopy) _outactors) (Variables|Default|GetAmountRooms)))