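; Spike trap actor that moves a cone spike vertically and damages the player character on contact.
; From BeginPlay, a timeline's SpikeHeight track sets the cone's relative Z without sweep, calling Play again on each update.
; The Damage_trigger overlap casts to BP_ThirdPersonCharacter, prints a debug message and calls the character's TakeDamage.
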(event OnComponentBeginOverlap(Damage_trigger)
  (params (OverlappedComponent :type Primitive%20Component%20Object%20Reference) (OtherActor :type Actor%20Object%20Reference) (OtherComp :type Primitive%20Component%20Object%20Reference) (OtherBodyIndex :type Integer) (bFromSweep :type Boolean) (SweepResult :type Hit%20Result%20Structure%20%28by%20ref%29))
  (bind _asbp_third_person_character (Utilities|Casting|CastToBP_ThirdPersonCharacter OtherActor))
  (Development|PrintString "DAMAGE 10")
  (Default|TakeDamage _asbp_third_person_character (Variables|Default|GetDamage10)))

(event Collision|EventActorBeginOverlap
  (params (OtherActor :type Actor%20Object%20Reference)))

(event EventTick
  (params (DeltaSeconds :type Float%20%28single-precision%29)))

(event EventBeginPlay
  (bind _cone (Variables|Default|GetCone))
  (bind _relativelocation (Variables|/Script/Engine.SceneComponent|GetRelativeLocation _cone))
  (bind (_x _y) (Math|Vector|BreakVector _relativelocation))
  (bind _spikeheight (Timeline|Шкала%20времени Play)
    (:Update
      (Transformation|SetRelativeLocation (Variables|Default|GetCone) (Math|Vector|MakeVector _x _y _spikeheight) false false)
      (Timeline|Шкала%20времени Play))))

(fn ConstructionScript)